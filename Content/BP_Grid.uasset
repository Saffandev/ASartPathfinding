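; BP_Grid is a navigation grid actor that displays nav tiles through a hierarchical instanced static mesh.
; On BeginPlay it waits briefly, calls CreateNavMesh, defined outside this file, then batch-adds instances from NodesTransforms.
; An older Blueprint builder, which box-traces cells for obstacles, creates nodes and links eight-way neighbours by flat-array index offsets, remains disconnected.
; The construction script is empty, and other debug and test snippets are unwired.
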(event `test`)

(event `CustomEvent_0`
  (`AddComponent|NODE_AddStaticMeshComponent-0` :`RelativeTransform` (`KismetMathLibrary.MakeTransform` (0.0 0.0 0.0) (struct) (10.0 10.0 10.0))))

(event `self.ReceiveTick`
  (params (DeltaSeconds :type "Float (single-precision)")))

(event `Generate`)

(event `self.ReceiveBeginPlay`
  (`KismetSystemLibrary.Delay` 2.0)
  (`self.CreateNavMesh`)
  (`InstancedStaticMeshComponent.AddInstances` (`self.HierarchicalInstancedStaticMesh`) (`self.NodesTransforms`) false false))

(event `self.AddInstance`
  (params (Transform :type "Transform Structure")))

(fn `AddNeighbourNodes`
  (locals (Index :type Integer))
  (for (_array_element _array_index) (`self.GridArray`)
    (`KismetArrayLibrary.Array_Clear` (`self.LocalNeighbourNode`))
    (`/Engine/EditorBlueprintResources/StandardMacros.IsValid` _array_element
      (:`Is Valid`
        (set `local.Index` _array_index)
        ;[1 1 1] Down
        (`self.AddValidNeighbourNode` (+ (`local.Index`) (`self.Size_Y`) 0))
        ;[1 1 1] Up
        (`self.AddValidNeighbourNode` (+ (- (`local.Index`) (`self.Size_Y`)) 0))
        ;[1 1 1] Prev
        (`self.AddValidNeighbourNode` (- (`local.Index`) 1))
        ;[1 1 1] next
        (`self.AddValidNeighbourNode` (+ (`local.Index`) 1))
        ;[1 1 1] BottomRight
        (`self.AddValidNeighbourNode` (+ (`local.Index`) (`self.Size_Y`) -1))
        ;[1 1 1] upLeft
        (`self.AddValidNeighbourNode` (+ (- (`local.Index`) (`self.Size_Y`)) 1))
        ;[1 1 1] BottomLeft
        (`self.AddValidNeighbourNode` (+ (`local.Index`) (`self.Size_Y`) 1))
        ;[1 1 1] UpRight
        (`self.AddValidNeighbourNode` (+ (- (`local.Index`) (`self.Size_Y`)) -1))
        (set `NavNodes.NeighbourNode` (`self.LocalNeighbourNode`) _array_element)))))

(fn `AddValidNeighbourNode`
  (params (A :type Integer))
  (bind _output (`|GetArrayItem` (`self.GridArray`) A))
  (if (> A 0)
    (`/Engine/EditorBlueprintResources/StandardMacros.IsValid` _output
      (:`Is Valid`
        (`KismetArrayLibrary.Array_Add` (`self.LocalNeighbourNode`) _output)))))

(fn `CalculateIndexBP`
  (params (X :type Integer) (Y :type Integer))
  (returns (ReturnValue :type Integer))
  (return (+ (* (`self.Size_Y`) X) Y)))

(fn `SetArrayElement`
  (params (x :type Integer) (y :type Integer) (Item :type "Vector Structure (by ref)"))
  (locals (`LocalNavNode]` :type "NavNodes Object Reference"))
  (`self.CreateNavNode` (`self.CalculateIndex` x y) (`KismetMathLibrary.TransformLocation` (`self.GetTransform`) Item)))

(fn `UserConstructionScript`
  (locals (NewLocalVar_0 :type "Array of Actor Object Reference")))