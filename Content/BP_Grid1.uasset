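; Grid pathfinding actor that builds a tile map around obstacles and runs A* between chosen start and end nodes.
; Construction script box-traces each cell, hiding blocked tiles as zero-scale HISM instances and creating indexed NavNodes objects for open ones.
; BeginPlay links four-way neighbours by flat-index offsets.
; AStar uses squared distances and a bubble-sorted open list; DrawPath's parent-tracing debug draw is disconnected.
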(event `self.ReceiveTick`
  (params (DeltaSeconds :type "Float (single-precision)")))

(event `self.ReceiveBeginPlay`
  (`self.AddNeighbourNodes`))

(event `Generate`)

(fn `AddNeighbourNodes`
  (locals (Index :type Integer))
  (for (_array_element _array_index) (`self.GridArray`)
    (`KismetArrayLibrary.Array_Clear` (`self.LocalNeighbourNode`))
    (`/Engine/EditorBlueprintResources/StandardMacros.IsValid` _array_element
      (:`Is Valid`
        (set `local.Index` _array_index)
        ;[1 1 1] Down
        (`self.AddValidNeighbourNode` (+ (`local.Index`) (`self.Size_Y`) 0))
        ;[1 1 1] Up
        (`self.AddValidNeighbourNode` (+ (- (`local.Index`) (`self.Size_Y`)) 0))
        ;[1 1 1] Prev
        (`self.AddValidNeighbourNode` (- (`local.Index`) 1))
        ;[1 1 1] next
        (`self.AddValidNeighbourNode` (+ (`local.Index`) 1))
        (set `NavNodes.NeighbourNode` (`self.LocalNeighbourNode`) _array_element)))))

(fn `AddValidNeighbourNode`
  (params (A :type Integer))
  (bind _output (`|GetArrayItem` (`self.GridArray`) A))
  (if (> A 0)
    (`/Engine/EditorBlueprintResources/StandardMacros.IsValid` _output
      (:`Is Valid`
        (`KismetArrayLibrary.Array_Add` (`self.LocalNeighbourNode`) _output)))))

(fn `AStar`
  (locals (LocalNeighbourNode :type "NavNodes Object Reference") (LocalNeighbourLocalGoal :type "Float (double-precision)" :default 0.0))
  (for _array_element (`self.GridArray`)
    (`/Engine/EditorBlueprintResources/StandardMacros.IsValid` _array_element
      (:`Is Valid`
        (`NavNodes.Reset` _array_element))))
  (`/Engine/EditorBlueprintResources/StandardMacros.IsValid` (`self.NodeStart`)
    (:`Is Valid`
      (`/Engine/EditorBlueprintResources/StandardMacros.IsValid` (`self.NodeEnd`)
        (:`Is Valid`
          (`self.SetCurrentNode`)
          (`KismetArrayLibrary.Array_Clear` (`self.NonTestedNodes`))
          (`KismetArrayLibrary.Array_Add` (`self.NonTestedNodes`) (`self.CurrentNode`))
          (while (and (`KismetArrayLibrary.Array_IsNotEmpty` (`self.NonTestedNodes`)) (!= (`self.CurrentNode`) (`self.NodeEnd`)))
            (bind _node_group1 (`self.SortNodeGroup` (`self.NonTestedNodes`)))
            (set `self.NonTestedNodes` _node_group1)
            (while (and (`KismetArrayLibrary.Array_IsNotEmpty` (`self.NonTestedNodes`)) (`NavNodes.bIsVisited` (`|GetArrayItem` (`self.NonTestedNodes`))))
              (`KismetArrayLibrary.Array_Remove` (`self.NonTestedNodes`)))
            (if (`KismetArrayLibrary.Array_IsEmpty` (`self.NonTestedNodes`))
              (`self.DrawPath`)
              (return)
              (else
                (bind _output_get (set `self.CurrentNode` (`|GetArrayItem` (`self.NonTestedNodes`))))
                (set `NavNodes.bIsVisited` true _output_get)
                (for _array_element_2 (`NavNodes.NeighbourNode` (`self.CurrentNode`))
                  (`/Engine/EditorBlueprintResources/StandardMacros.IsValid` _array_element_2
                    (:`Is Valid`
                      (`KismetSystemLibrary.DrawDebugSphere` (`NavNodes.NodeLoc` (stale _output_get_2)) 20.0 12 (struct :`A` 1.0) 1.0)
                      (bind _output_get_2 (set `local.LocalNeighbourNode` _array_element_2))
                      (if (not (`NavNodes.bIsVisited` (`local.LocalNeighbourNode`)))
                        (`KismetArrayLibrary.Array_Add` (`self.NonTestedNodes`) (`local.LocalNeighbourNode`)))
                      (set `local.LocalNeighbourLocalGoal` (`self.CaculateDistance` (`self.CurrentNode`) (`local.LocalNeighbourNode`)))
                      (if (< (+ (`local.LocalNeighbourLocalGoal`) (`NavNodes.LocalGoal` (`self.CurrentNode`))) (`NavNodes.LocalGoal` (`local.LocalNeighbourNode`)))
                        (set `NavNodes.ParentNode` (`self.CurrentNode`) (`local.LocalNeighbourNode`))
                        (set `NavNodes.LocalGoal` (`local.LocalNeighbourLocalGoal`) (`local.LocalNeighbourNode`))
                        (set `NavNodes.GloablGoal` (+ (`NavNodes.LocalGoal` (`local.LocalNeighbourNode`)) (`self.CaculateDistance` (`local.LocalNeighbourNode`) (`self.NodeEnd`))) (`local.LocalNeighbourNode`)))))))))
          (`self.DrawPath`)
          (return))
        (:`Is Not Valid`
          (`KismetSystemLibrary.PrintString` "----------No End Node----------" true true (struct :`B` 1.0 :`A` 1.0)))))
    (:`Is Not Valid`
      (`KismetSystemLibrary.PrintString` "----------No Star Node----------" true true (struct :`R` 1.0 :`A` 1.0)))))

(fn `CaculateDistance`
  (params (`node A` :type "NavNodes Object Reference") (`node B` :type "NavNodes Object Reference"))
  (returns (ReturnValue :type "Float (double-precision)"))
  (return (`KismetMathLibrary.Vector_DistanceSquared` (`NavNodes.NodeLoc` (`local.node A`)) (`NavNodes.NodeLoc` (`local.node B`)))))

(fn `CalculateIndex`
  (params (X :type Integer) (Y :type Integer))
  (returns (ReturnValue :type Integer))
  (return (+ (* (`self.Size_Y`) X) Y)))

(fn `DrawPath`
  (`self.NodeEnd`
    (:`then`
      (set `self.DrawingNode` (`self.NodeEnd`)))
    (:`else`
      (`KismetSystemLibrary.PrintString` "end node not valid when drawing the path"))))

(fn `SetArrayElement`
  (params (x :type Integer) (y :type Integer) (Item :type "Vector Structure (by ref)"))
  (locals (`LocalNavNode]` :type "NavNodes Object Reference"))
  (bind _returnvalue (`self.CalculateIndex` x y))
  (bind _localnavnode_ (`local.LocalNavNode]`))
  (bind _returnvalue_2 (`AddComponent|NODE_AddTextRenderComponent-2` :`RelativeTransform` (`KismetMathLibrary.MakeTransform` (+ Item (0.0 0.0 10.0)) (struct :`Pitch` 90.0))))
  (`TextRenderComponent.K2_SetText` _returnvalue_2 (`KismetTextLibrary.Conv_IntToText` _returnvalue))
  (bind _returnvalue_3 (`|GenericCreateObject` "/Script/ASartPathfinding.NavNodes"))
  (set `local.LocalNavNode]` _returnvalue_3)
  (set `NavNodes.bIsVisited` false _localnavnode_)
  (set `NavNodes.ParentNode` null _localnavnode_)
  (set `NavNodes.NodeLoc` (`KismetMathLibrary.TransformLocation` (`self.GetTransform`) (`local.Item`)) _localnavnode_)
  (`KismetArrayLibrary.Array_Set` (`self.GridArray`) _returnvalue (`local.LocalNavNode]`)))

(fn `SetCurrentNode`
  (bind _nodestart (`self.NodeStart`))
  (set `NavNodes.LocalGoal` 0.0 _nodestart)
  (set `NavNodes.GloablGoal` (`self.CaculateDistance` (`self.NodeStart`) (`self.NodeEnd`)) _nodestart)
  (set `self.CurrentNode` (`self.NodeStart`)))

(fn `SetEndNode`
  (params (Index :type Integer))
  (bind _output_get (set `self.NodeEnd` (`|GetArrayItem` (`self.GridArray`) Index)))
  (`KismetSystemLibrary.DrawDebugSphere` (`NavNodes.NodeLoc` _output_get) 40.0 12 (struct :`R` 0.470833 :`G` 0.034244 :`A` 1.0) 5.0 3.0))

(fn `SetStartNode`
  (params (Index :type Integer))
  (bind _output (`|GetArrayItem` (`self.GridArray`) Index))
  (`/Engine/EditorBlueprintResources/StandardMacros.IsValid` _output
    (:`Is Valid`
      (bind _output_get (set `self.NodeStart` _output))
      (`KismetSystemLibrary.DrawDebugSphere` (`NavNodes.NodeLoc` _output_get) 40.0 12 (struct :`R` 0.277047 :`B` 0.470833 :`A` 1.0) 5.0 3.0))))

(fn `SortNodeGroup`
  (params (`Node Group` :type "Array of NavNodes Object Reference"))
  (returns (`Node Group1` :type "Array of NavNodes Object Reference"))
  (bind _returnvalue (`KismetArrayLibrary.Array_Length` `Node Group`))
  (bind _returnvalue_2 (- _returnvalue 1))
  (if (> _returnvalue 1)
    (for _index (range (+ _returnvalue_2 1))
      (for _index_2 (range (+ (- _returnvalue_2 _index 1) 1))
        (bind _returnvalue_3 (+ _index_2 1))
        (if (> (`NavNodes.GloablGoal` (`|GetArrayItem` (`local.Node Group`) _index_2)) (`NavNodes.GloablGoal` (`|GetArrayItem` (`local.Node Group`) _returnvalue_3)))
          (`KismetArrayLibrary.Array_Swap` (`local.Node Group`) _index_2 _returnvalue_3)))))
  (return (`local.Node Group`)))

(fn `UserConstructionScript`
  (locals (NewLocalVar_0 :type "Array of Actor Object Reference"))
  (bind _instance_transform_location (`self.Instance Transform Location`))
  (bind (_instance_transform_location_x _instance_transform_location_y _instance_transform_location_z) (`KismetMathLibrary.BreakVector` (`self.Instance Transform Location`)))
  (bind (_instance_transform_location_x_2 _instance_transform_location_y_2 _instance_transform_location_z_2) (`KismetMathLibrary.BreakVector` (`self.Instance Transform Location`)))
  (bind _returnvalue (`KismetMathLibrary.TransformLocation` (`self.GetTransform`) (`self.Instance Transform Location`)))
  (bind (_returnvalue_origin _returnvalue_boxextent) (`KismetMathLibrary.BreakBoxSphereBounds` (`StaticMesh.GetBounds` (`StaticMeshComponent.StaticMesh` (`self.HierarchicalInstancedStaticMesh`)))))
  (bind (_returnvalue_origin_2 _returnvalue_boxextent_2) (`KismetMathLibrary.BreakBoxSphereBounds` (`StaticMesh.GetBounds` (`StaticMeshComponent.StaticMesh` (`self.HierarchicalInstancedStaticMesh`)))))
  (bind (_returnvalue_origin_3 _returnvalue_boxextent_3) (`KismetMathLibrary.BreakBoxSphereBounds` (`StaticMesh.GetBounds` (`StaticMeshComponent.StaticMesh` (`self.HierarchicalInstancedStaticMesh`)))))
  (bind (_x _y _z) (`KismetMathLibrary.BreakVector3f` _returnvalue_boxextent))
  (`KismetArrayLibrary.Array_Resize` (`self.GridArray`) (* (`self.Size_X`) (`self.Size_Y`)))
  ;[0.2052 0.2052 0.2052] Creating Grid
  ;;[0.2052 0.2052 0.2052] Creating Grid
  ;;;[1 1 1] XLocation
  (for _index (range (`self.Size_X`))
    (set `self.XIndex` _index)
    (set `self.Instance Transform Location` (`KismetMathLibrary.MakeVector` (* _index (`KismetMathLibrary.BreakVector3f` _returnvalue_boxextent_2) 2.01) _instance_transform_location_y_2 _instance_transform_location_z_2))
    ;;;[1 1 1] YLocation
    (for _index_2 (range (`self.Size_Y`))
      (set `self.YIndex` _index_2)
      (set `self.Instance Transform Location` (`KismetMathLibrary.MakeVector` _instance_transform_location_x (* _index_2 (`.Y` (`KismetMathLibrary.BreakVector3f` _returnvalue_boxextent_3)) 2.01) _instance_transform_location_z))
      ;[1 1 1] Creating the nav tiles
      (bind (_outhit _returnvalue_2) (`KismetSystemLibrary.BoxTraceSingle` _returnvalue _returnvalue (`KismetMathLibrary.MakeVector` _x _y (/ _z 4.0)) (struct) "TraceTypeQuery1" false (`local.NewLocalVar_0`) "None" true (struct :`R` 1.0 :`A` 1.0) (struct :`G` 1.0 :`A` 1.0) 1.0))
      (if _returnvalue_2
        (`InstancedStaticMeshComponent.AddInstance` (`self.HierarchicalInstancedStaticMesh`) (`KismetMathLibrary.MakeTransform` (`self.Instance Transform Location`) (struct) (0.0 0.0 0.0)) false)
        (else
          (`InstancedStaticMeshComponent.AddInstance` (`self.HierarchicalInstancedStaticMesh`) (`KismetMathLibrary.MakeTransform` _instance_transform_location (struct) (1.0 1.0 0.3)) false)
          (`self.SetArrayElement` (`self.XIndex`) (`self.YIndex`) _instance_transform_location))))))